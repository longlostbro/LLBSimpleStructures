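; Display table structure that lets players place an allowed item from their inventory and pick it back up through multi-use menu entries.
; On the server, BeginPlay builds the allowed class list from a string, optionally from game mode options, and registers use indices per class.
; Placing stores the item as bytes and references its weapon mesh; pickup recreates it from those bytes.
; The SaveGame persistence logic is unconnected.
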(event EventBeginPlay
  (|CallParentFunction)
  (Utilities|FlowControl|RetriggerableDelay 0.2)
  (Utilities|SwitchNetAuthority
    (:DedicatedServer
      _)
    (:PlayerServer
      _))
  (Utilities|FlowControl|Sequence
    (:then_0
      (CallFunction|SetAllowedDisplayItems))
    (:then_1
      (CallFunction|RegisterDisplayableItemsMultiUseEntries))))

(fn ConstructionScript
  (|CallParentFunction))

(fn BPGetMultiUseEntries
  (params (ForPC :type Player%20Controller%20Object%20Reference) (MultiUseEntries :type Array%20of%20Multi%20Use%20Entry%20Structures))
  (bind _displayeditembytes (Variables|Default|GetDisplayedItemBytes))
  (bind _returnvalue (Utilities|Array|Length _displayeditembytes))
  (bind _returnvalue_2 (> _returnvalue 0))
  (bind _mu_entries (CallFunction|InitializeMUEntries MultiUseEntries))
  (LocalVariables|SetMU%20Buffer _mu_entries)
  (if (and (Utilities|IsValid (Variables|Default|GetDisplayedItem)) _returnvalue_2)
    (bind _mu_buffer_out (CallFunction|SetEntryforGetItem (LocalVariables|GetMU%20Buffer) :!label _label))
    (LocalVariables|SetMU%20Buffer _mu_buffer_out)
    (else
      (if _returnvalue_2
        (bind _returnvalue_3 (Class|PrimalItem|CreatefromBytes _displayeditembytes))
        (if (Utilities|IsValid _returnvalue_3)
          (Variables|Default|SetDisplayedItem _returnvalue_3)
          (goto _label)
          (else
            (Development|PrintString "failed to create item from bytes")))
        (else
          (Development|PrintString "no item bytes saved")))
      (Development|PrintString "Failed to find item in table")
      (bind _mu_buffer_out_2 (CallFunction|SetEntriesforPlacingItem ForPC (LocalVariables|GetMU%20Buffer)))
      (LocalVariables|SetMU%20Buffer _mu_buffer_out_2)))
  (return (LocalVariables|GetMU%20Buffer)))

(fn BPTryMultiUse
  (params (ForPC :type Player%20Controller%20Object%20Reference) (UseIndex :type Integer))
  (Class|PrimalStructure|BPGetStructureID self)
  (bind _asshooterplayercontroller (Utilities|Casting|CastToShooterPlayerController ForPC))
  (if (> (Utilities|Array|Length (Variables|Default|GetDisplayedItemBytes)) 0)
    (CallFunction|MoveDisplayedItemtoPlayer (Variables|/Script/ShooterGame.PrimalCharacter|GetMyInventoryComponent (Class|ShooterPlayerController|GetPlayerCharacter _asshooterplayercontroller)))
    (else
      (bind _primal_item_class (CallFunction|GetDisplayItemfromRegistry UseIndex))
      (CallFunction|MovePlayerItemtoDisplayTable (Variables|/Script/ShooterGame.PrimalCharacter|GetMyInventoryComponent (Class|ShooterPlayerController|GetPlayerCharacter _asshooterplayercontroller)) _primal_item_class)))
  (return true))

(fn StringtoPrimalItemClasses
  (params (stringOfBlueprints :type String) (delimiter :type String) (cullEmptyStrings :type Boolean) (clearItems :type Boolean) (inputPrimalItems :type Array%20of%20Primal%20Item%20Class%20References))
  (bind _returnvalue (Utilities|String|ParseIntoArray stringOfBlueprints delimiter cullEmptyStrings))
  (if (> (Utilities|Array|Length _returnvalue) 0)
    (if clearItems
      (Utilities|Array|Clear inputPrimalItems))
    (for _array_element _returnvalue
      (bind _returnvalue_2 (Class|VictoryCore|BPLoadClass _array_element))
      (bind _asprimalitem (Utilities|Casting|CastToPrimalItemClass _returnvalue_2))
      (Utilities|Array|Add inputPrimalItems _asprimalitem))
    (return inputPrimalItems)))

(fn InitializeMUEntries
  (params (Initial%20MU%20Entries :type Array%20of%20Multi%20Use%20Entry%20Structures))
  (LocalVariables|SetMU%20Buffer Initial%20MU%20Entries)
  (for _array_element (LocalVariables|GetMU%20Buffer)
    (if true
      (Utilities|Array|RemoveItem (LocalVariables|GetMU%20Buffer) _array_element)))
  (return (LocalVariables|GetMU%20Buffer)))

(fn MakeGetEntry
  (params (ItemDisplayed :type Primal%20Item%20Object%20Reference))
  (return (Utilities|Struct|MakeMultiUseEntry 0 (Utilities|String|Append "Pickup " (Utilities|GetDisplayName ItemDisplayed)) 9844)))

(fn SetAllowedDisplayItems
  (bind _asshootergamemode (Utilities|Casting|CastToShooterGameMode (Game|GetGameMode))
    (:then
      (if (Variables|Default|GetbGetItemsFromOptions)
        (bind _returnvalue (Class|ShooterGameMode|GetStringOption _asshootergamemode "LLBSimpleStructures" "DisplayableItems"))
        (Variables|Default|SetstringDisplayableItems _returnvalue))
      (bind _outputprimalitems (CallFunction|StringtoPrimalItemClasses self (Variables|Default|GetstringDisplayableItems) "," true false (Variables|Default|GetDisplayableItems)))
      (Variables|Default|SetDisplayableItems _outputprimalitems))
    (:CastFailed
      _))
  (return))

(fn RegisterDisplayableItemsMultiUseEntries
  (for (_array_element _array_index) (Variables|Default|GetDisplayableItems)
    (CallFunction|RegisterDisplayableItemMultiUseEntry _array_index _array_element))
  (Variables|Default|SetDisplayItemRegistry (Variables|Default|GetDisplayItemRegistry) true)
  (Variables|Default|SetDisplayItems (Variables|Default|GetDisplayItems) true)
  (return))

(fn RegisterDisplayableItemMultiUseEntry
  (params (index :type Integer) (Primal%20Item%20Class :type Primal%20Item%20Class%20Reference))
  (bind _returnvalue (+ index 9845))
  (bind _returnvalue_2 (Utilities|Array|Add (Variables|Default|GetDisplayItemRegistry) _returnvalue))
  (Utilities|Array|SetArrayElem (Variables|Default|GetDisplayItems) _returnvalue_2 (Utilities|Struct|MakeDisplayItemStruct (Utilities|GetClassDisplayName Primal%20Item%20Class) (Class|VictoryCore|GetClassString Primal%20Item%20Class) Primal%20Item%20Class _returnvalue) true))

(fn GetDisplayItemfromRegistry
  (params (ItemToFind :type Integer%20%28by%20ref%29))
  (return (.ItemClass (Utilities|Struct|BreakDisplayItemStruct (Utilities|Array|Get(acopy) (Variables|Default|GetDisplayItems) (Utilities|Array|FindItem (Variables|Default|GetDisplayItemRegistry) ItemToFind))))))

(fn MoveDisplayedItemtoPlayer
  (params (PlayerInventoryComponent :type Primal%20Inventory%20Component%20Object%20Reference))
  (bind _returnvalue (Class|PrimalItem|CreatefromBytes (Variables|Default|GetDisplayedItemBytes)))
  (bind _asprimalitem_base_c (Utilities|Casting|CastToPrimalItem_Base _returnvalue))
  (Class|PrimalInventoryComponent|AddItemObject PlayerInventoryComponent _asprimalitem_base_c)
  (Variables|Default|SetDisplayedItemMesh 0)
  (Utilities|Array|Clear (Variables|Default|GetDisplayedItemBytes))
  (Variables|Default|SetDisplayedItemBytes (Variables|Default|GetDisplayedItemBytes) true))

(fn MovePlayerItemtoDisplayTable
  (params (Players%20Inventory%20Component :type Primal%20Inventory%20Component%20Object%20Reference) (PrimalItemClass :type Primal%20Item%20Class%20Reference))
  (bind _returnvalue (Class|PrimalInventoryComponent|FindAllItemsOfType Players%20Inventory%20Component PrimalItemClass false true true false true false false))
  (if (> (Utilities|Array|Length _returnvalue) 0)
    (bind _bytes (Class|PrimalItem|GetItemBytes (Utilities|Array|Get(acopy) _returnvalue)))
    (Variables|Default|SetDisplayedItemBytes _bytes true)
    (CallFunction|UpdateDisplayableItemMesh (Utilities|Array|Get(acopy) _returnvalue))
    (Class|PrimalInventoryComponent|RemoveItem Players%20Inventory%20Component (Variables|/Script/ShooterGame.PrimalItem|GetItemID (Utilities|Array|Get(acopy) _returnvalue)) false false false true)))

(fn UpdateDisplayableItemMesh
  (params (PrimalItemReference :type Primal%20Item%20Object%20Reference))
  (bind (_mesh3p _skeletalmesh) (Utilities|GetMeshfromWeapon PrimalItemReference))
  (Variables|Default|SetDisplayedItemMesh _mesh3p)
  (Class|SkinnedMeshComponent|SetSkeletalMesh (Variables|Default|GetDisplayedItemMesh) _skeletalmesh)
  (return))

(fn SetEntriesforPlacingItem
  (params (PC :type Player%20Controller%20Object%20Reference) (MU%20Buffer%20In :type Array%20of%20Multi%20Use%20Entry%20Structures))
  (bind _asshooterplayercontroller (Utilities|Casting|CastToShooterPlayerController PC)
    (:then
      (for _array_element (Variables|Default|GetDisplayItems)
        (bind _returnvalue (Class|PrimalInventoryComponent|FindAllItemsOfType (Variables|/Script/ShooterGame.PrimalCharacter|GetMyInventoryComponent (Class|ShooterPlayerController|GetPlayerCharacter _asshooterplayercontroller)) (.ItemClass (Utilities|Struct|BreakDisplayItemStruct _array_element)) false true true false true false false))
        (if (> (Utilities|Array|Length _returnvalue) 0)
          (Utilities|Array|Add MU%20Buffer%20In (Utilities|Struct|MakeMultiUseEntry 0 (Utilities|String|Append "Place " (.ItemName (Utilities|Struct|BreakDisplayItemStruct _array_element))) (.MultiUseIndex (Utilities|Struct|BreakDisplayItemStruct _array_element)))))
        (return MU%20Buffer%20In)))
    (:CastFailed
      _))
  (return MU%20Buffer%20In))

(fn SetEntryforGetItem
  (params (MU%20Buffer%20In :type Array%20of%20Multi%20Use%20Entry%20Structures))
  (Utilities|Array|Add MU%20Buffer%20In (Utilities|Struct|MakeMultiUseEntry 0 (Utilities|String|Append "Pickup " (Utilities|GetDisplayName (Variables|Default|GetDisplayedItem))) 9844))
  (return MU%20Buffer%20In))